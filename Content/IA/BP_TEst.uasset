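; Test Blueprint that tracks the direction from its own location to a Target actor, storing it without applying it.
; Each Tick, if Target is valid, it combines the look-at yaw with the look-at pitch fed in as roll.
; The same result is written to both Rotator and RotatorToEnemies.
; Unconnected nodes that read the Target mesh's "cabin" bone location remain in the graph.
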(event EventTick
  (params (DeltaSeconds :type Float%20%28single-precision%29))
  (bind _returnvalue (Transformation|GetActorLocation))
  (bind _returnvalue_2 (Transformation|GetActorLocation))
  (bind _target (Variables|Default|GetTarget))
  (bind _target_2 (Variables|Default|GetTarget))
  (bind _returnvalue_3 (Transformation|GetActorLocation _target_2))
  (bind _returnvalue_4 (Transformation|GetActorLocation _target))
  (bind _returnvalue_5 (Math|Rotator|FindLookatRotation _returnvalue_2 _returnvalue_4))
  (bind _returnvalue_6 (Math|Rotator|FindLookatRotation _returnvalue _returnvalue_3))
  (bind _returnvalue_7 (Math|Rotator|CombineRotators (Math|Rotator|MakeRotator 0.0 0.0 (.yaw _returnvalue_5)) (Math|Rotator|MakeRotator (.pitch _returnvalue_6) 0.0 0.0)))
  (Utilities|IsValid (Variables|Default|GetTarget)
    (:Is%20Valid
      (Variables|Default|SetRotator _returnvalue_7)
      (Variables|Default|SetRotatorToEnemies _returnvalue_7))))

(fn ConstructionScript)