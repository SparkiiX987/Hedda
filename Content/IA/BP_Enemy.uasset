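; Enemy Blueprint for an AI-controlled arena combatant that caches GM_Arena and its BP_AIController on BeginPlay.
; GoToZone checks game-mode zones, writing one whose free-zone check returns false to the Blackboard and entering it, but its EventGraph call is disconnected.
; SetFaction forces one fixed faction on the controller.
; GetIdealRange supplies fixed attack and defend radii, while other zone queries are stubs or unwired.
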(event EventBeginPlay
  (|CallParentFunction)
  (bind _asgm_arena (Utilities|Casting|CastToGM_Arena (Game|GetGameMode)))
  (Variables|Default|SetGameMode _asgm_arena)
  (bind _asbp_aicontroller (Utilities|Casting|CastToBP_AIController (AI|GetAIController self)))
  (Variables|Default|SetAIController _asbp_aicontroller))

(event Collision|EventActorBeginOverlap
  (params (OtherActor :type Actor%20Object%20Reference)))

(event EventTick
  (params (DeltaSeconds :type Float%20%28single-precision%29))
  (|CallParentFunction DeltaSeconds) ; This node is disabled and will not be called.\nDrag off pins to build functionality.
)

(fn ConstructionScript
  (|CallParentFunction))

(fn GotoZone
  (bind _aicontroller (Variables|Default|GetAIController))
  (bind _array_element (Utilities|Array|ForEachLoopwithBreak (Variables|/Game/GameModes/GM_Arena.GM_Arena_C|GetZone (Variables|Default|GetGameMode)) :!label _label)
    (:LoopBody
      (bind _bool (Class|BPIEnemyAI|GetFreeZone(Message) _array_element self))
      (Development|PrintString (Utilities|String|ToString(Boolean) _bool))
      (if _bool
        (goto _label)
        (else
          (AI|Components|Blackboard|SetValueasObject (AI|GetBlackboard _aicontroller) (Variables|/Game/IA/BP_AIController.BP_AIController_C|GetCurrentZone _aicontroller) _array_element)
          (Class|BPIEnemyAI|GoIntoZone(Message) _array_element self)
          (goto _label Break))))))

(fn SetFaction
  (params (Faction :type Faction%20Enum :default "NewEnumerator0"))
  (|CallParentFunction Faction)
  (Variables|/Game/IA/BP_AIController.BP_AIController_C|SetFaction (Variables|Default|GetAIController) "NewEnumerator0"))

(fn GetEnemiinZone
  (params (Self%20Actor :type C%20Base%20Character%20Object%20Reference))
  (return 0))

(fn GetFreeZone
  (params (Actor :type BP%20Enemy%20Object%20Reference))
  (return false 0))

(fn GetIdealRange
  (return 1.5e+02 5e+02))