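; Arena game mode for a two-team Mage vs Mecha match with AI and a selectable player character.
; On BeginPlay it spawns entities at spawn-manager points, fills factions, and assigns AI to zones through their blackboards.
; RespawnEntity replaces an entity, scores against its faction, and CheckPoints shows win or lose at a threshold.
; The match timer is disconnected, leaving its tie-break Last Stand unreached; obstacle moving is a print stub.
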(event EventBeginPlay
  (Variables|Default|SetobstacleMoveCooldown 15.0)
  (Variables|Default|Settimer 3e+02)
  (Variables|Default|SetfirstTeamPoints 0.0)
  (Variables|Default|SetsecondTeamPoints 0.0)
  (CallFunction|SpawnEntity)
  (CallFunction|AssignZone))

(event EventTick
  (params (DeltaSeconds :type Float%20%28single-precision%29)))

(fn ConstructionScript)

(fn SpawnPlayer
  (params (_position :type Vector))
  (Game|SpawnActorfromClass "/Game/Character/Player/Blueprint/C_PlayerCharacter.C_PlayerCharacter_C" (Math|Transform|MakeTransform _position "0, 0, 0" "1.000000,1.000000,1.000000") "Undefined" "MultiplyWithRoot" 0 0))

(fn SpawnEntity
  (bind _outactors (Actor|GetAllActorsOfClass "/Game/Zone/BP_Zone.BP_Zone_C"))
  (Variables|Default|SetZone _outactors)
  (bind _returnvalue (Actor|GetActorOfClass "/Game/Zone/BP_SpawnPointManager.BP_SpawnPointManager_C"))
  (Variables|Default|SetOut%20Actors (Variables|/Game/Zone/BP_SpawnPointManager.BP_SpawnPointManager_C|GetSpawnPoints _returnvalue))
  (if (Variables|Default|GetbDebug)
    (for _index (range 0 (- (Variables|Default|GetNumberOfAI) 1))
      (CallFunction|SpawnAI (Utilities|Array|Get(acopy) (Variables|Default|GetOut%20Actors) _index)))
    (CallFunction|AssignZone)
    (else
      (for _index_2 (range 0 (- (Variables|Default|GetNumberOfAI) 1))
        (if (!= _index_2 0)
          (CallFunction|SpawnAI (Utilities|Array|Get(acopy) (Variables|Default|GetOut%20Actors) _index_2))
          (else
            (bind _asgi_select_game_instance (Utilities|Casting|CastToGI_SelectGameInstance (Game|GetGameInstance)))
            (bind _returnvalue_2 (Game|SpawnActorfromClass (Variables|/Game/Save/Blueprint/GI_SelectGameInstance.GI_SelectGameInstance_C|GetcharChoice _asgi_select_game_instance) (Math|Transform|MakeTransform (Transformation|GetActorLocation (Utilities|Array|Get(acopy) (Variables|Default|GetOut%20Actors) _index_2)) "0, 0, 0" "1.000000,1.000000,1.000000") "AlwaysSpawn" "MultiplyWithRoot" 0 0))
            (bind _asc_base_character (Utilities|Casting|CastToC_BaseCharacter _returnvalue_2))
            (Pawn|Possess (Game|GetPlayerController 0) _asc_base_character)
            (CallFunction|SetFaction _asc_base_character))))
      (CallFunction|AssignZone))))

(fn DisplayResultGame
  (params (_firstTeamWon :type Boolean))
  (if _firstTeamWon
    (bind _returnvalue (UserInterface|CreateWidget "/Game/Menus/Blueprints/UW_Win.UW_Win_C"))
    (UserInterface|Viewport|AddtoViewport _returnvalue 0)
    (Audio|PlaySound2D "/Game/SoundManager/SFX/Endings/Victory/SSC_dark-chords-103048.SSC_dark-chords-103048" 1.0 1.0 0.0 0 0)
    (else
      (bind _returnvalue_2 (UserInterface|CreateWidget "/Game/Menus/Blueprints/UW_Lose.UW_Lose_C"))
      (UserInterface|Viewport|AddtoViewport _returnvalue_2 0)
      (Audio|PlaySound2D "/Game/SoundManager/SFX/Endings/Defeat/SSC_defeat-background-39613.SSC_defeat-background-39613" 1.0 1.0 0.0 0 0)))
  (Variables|/Script/Engine.PlayerController|SetbShowMouseCursor (Game|GetPlayerController 0) true))

(fn MoveObstacles
  (Variables|Default|SetobstacleMoveCooldown 15.0)
  (Development|PrintText "MoveObstacle"))

(fn DecrementCooldown
  (params (_obstacleCoolDown :type Float%20%28double-precision%29) (_deltaTime :type Float%20%28double-precision%29))
  (Variables|Default|SetobstacleMoveCooldown (- _obstacleCoolDown _deltaTime)))

(fn DecrementTimer
  (params (_gameTime :type Float%20%28double-precision%29) (_deltaTime :type Float%20%28double-precision%29))
  (bind _output_get (Variables|Default|Settimer (- _gameTime _deltaTime)))
  (if (<= _output_get 0.0)
    (CallFunction|MoveObstacles)))

(fn StartLastStandMode
  (Variables|Default|SetbLastStandModeActivated true)
  (bind _outactors (Actor|GetAllActorsOfClass "/Game/Character/C_BaseCharacter.C_BaseCharacter_C"))
  (bind _output_get (Variables|Default|SetPlayers _outactors))
  (for _array_element _output_get
    (Actor|DestroyActor _array_element))
  (CallFunction|SpawnPlayer "0, 0, 0")
  (Game|SpawnActorfromClass "/Game/Character/C_BaseCharacter.C_BaseCharacter_C" (Math|Transform|MakeTransform "1000.000000,0.000000,0.000000" "0.000000,180.000000,0.000000" "1.000000,1.000000,1.000000") "Undefined" "MultiplyWithRoot" 0 0))

(fn CompareTeamsPoints
  (if (== (Variables|Default|GetfirstTeamPoints) (Variables|Default|GetsecondTeamPoints))
    (CallFunction|StartLastStandMode)
    (else
      (CallFunction|DisplayResultGame (> (Variables|Default|GetfirstTeamPoints) (Variables|Default|GetsecondTeamPoints))))))

(fn AssignZone
  (LocalVariables|SetLoopedAI2 0)
  (for _array_element (Variables|Default|GetEnemies)
    (LocalVariables|SetLooppedAI _array_element)
    (bind _array_element_2 (Utilities|Array|ForEachLoopwithBreak (Variables|Default|GetZone) :!label _label)
      (:LoopBody
        (LocalVariables|SetLooppedZone _array_element_2)
        (if (== (Utilities|Array|Length (Variables|/Game/Zone/BP_Zone.BP_Zone_C|GetEntity (LocalVariables|GetLooppedZone))) 0)
          (AI|Components|Blackboard|SetValueasObject (AI|GetBlackboard (Variables|/Game/IA/BP_Enemy.BP_Enemy_C|GetAIController (LocalVariables|GetLooppedAI))) (Variables|/Game/IA/BP_AIController.BP_AIController_C|GetCurrentZone (Variables|/Game/IA/BP_Enemy.BP_Enemy_C|GetAIController (LocalVariables|GetLooppedAI))) (LocalVariables|GetLooppedZone))
          (Variables|Default|SetLoopped%20AI2 (LocalVariables|GetLooppedAI))
          (Variables|/Game/Character/C_BaseCharacter.C_BaseCharacter_C|SetCurrentZone (LocalVariables|GetLooppedAI) (LocalVariables|GetLooppedZone))
          (Default|GoIntoZone (LocalVariables|GetLooppedZone) (LocalVariables|GetLooppedAI))
          (goto _label Break)
          (elif (and (< (Utilities|Array|Length (Variables|/Game/Zone/BP_Zone.BP_Zone_C|GetEntity (LocalVariables|GetLooppedZone))) 2) (Utilities|Enum|NotEqual(Enum) (Default|GetFaction (LocalVariables|GetLooppedAI)) (Default|GetFaction (Variables|Default|GetLoopped%20AI2))))
            (AI|Components|Blackboard|SetValueasObject (AI|GetBlackboard (Variables|/Game/IA/BP_Enemy.BP_Enemy_C|GetAIController (LocalVariables|GetLooppedAI))) (Variables|/Game/IA/BP_AIController.BP_AIController_C|GetCurrentZone (Variables|/Game/IA/BP_Enemy.BP_Enemy_C|GetAIController (LocalVariables|GetLooppedAI))) (LocalVariables|GetLooppedZone))
            (Default|GoIntoZone (LocalVariables|GetLooppedZone) (LocalVariables|GetLooppedAI))
            (Variables|/Game/Character/C_BaseCharacter.C_BaseCharacter_C|SetCurrentZone (LocalVariables|GetLooppedAI) (LocalVariables|GetLooppedZone))
            (goto _label Break)))))))

(fn SpawnAI
  (params (SpawnTransform_Location :type BP%20Spawn%20Point%20Object%20Reference))
  (bind _returnvalue (Game|SpawnActorfromClass "/Game/IA/BP_Enemy.BP_Enemy_C" (Math|Transform|MakeTransform (Transformation|GetActorLocation SpawnTransform_Location) "0, 0, 0" "1.000000,1.000000,1.000000") "AlwaysSpawn" "MultiplyWithRoot" 0 0))
  (Utilities|Array|Add (Variables|Default|GetEnemies) _returnvalue)
  (Variables|/Game/Character/C_BaseCharacter.C_BaseCharacter_C|SetSpawnPoint _returnvalue SpawnTransform_Location)
  (CallFunction|SetFaction _returnvalue))

(fn SetFaction
  (params (SpawnedObject :type C%20Base%20Character%20Object%20Reference))
  (if (< (Utilities|Array|Length (Variables|Default|GetFactionMage)) (Variables|Default|GetCountTeam1))
    (Default|SetFaction SpawnedObject "NewEnumerator0")
    (Utilities|Array|Add (Variables|Default|GetFactionMage) SpawnedObject)
    (elif (< (Utilities|Array|Length (Variables|Default|GetFactionMecha)) (Variables|Default|GetCountTeam2))
      (Default|SetFaction SpawnedObject "NewEnumerator1")
      (Utilities|Array|Add (Variables|Default|GetFactionMecha) SpawnedObject))))

(fn RespawnEntity
  (params (Entity :type C%20Base%20Character%20Object%20Reference))
  (LocalVariables|SetFaction (Default|GetFaction Entity))
  (LocalVariables|SetSpawnPoint (Variables|/Game/Character/C_BaseCharacter.C_BaseCharacter_C|GetSpawnPoint Entity))
  (bind _asbp_enemy (Utilities|Casting|CastToBP_Enemy Entity)
    (:then
      (bind _spawnpoint (LocalVariables|GetSpawnPoint)
        (:then
          (bind _returnvalue (Game|SpawnActorfromClass (Utilities|GetClass _asbp_enemy) (Math|Transform|MakeTransform (Transformation|GetActorLocation _spawnpoint) "0, 0, 0" "1.000000,1.000000,1.000000") "Undefined" "MultiplyWithRoot" 0 0))
          (Default|SetFaction _returnvalue (LocalVariables|GetFaction)))
        (:else)))
    (:CastFailed
      (bind _spawnpoint_2 (LocalVariables|GetSpawnPoint)
        (:then
          (bind _asgi_select_game_instance (Utilities|Casting|CastToGI_SelectGameInstance (Game|GetGameInstance)))
          (bind _returnvalue_2 (Game|SpawnActorfromClass (Variables|/Game/Save/Blueprint/GI_SelectGameInstance.GI_SelectGameInstance_C|GetcharChoice _asgi_select_game_instance) (Math|Transform|MakeTransform (Transformation|GetActorLocation _spawnpoint_2) "0, 0, 0" "1.000000,1.000000,1.000000") "Undefined" "MultiplyWithRoot" 0 0))
          (bind _asc_base_character (Utilities|Casting|CastToC_BaseCharacter _returnvalue_2))
          (Default|SetFaction _asc_base_character (LocalVariables|GetFaction)))
        (:else))))
  (Actor|DestroyActor Entity)
  (|SetScores (LocalVariables|GetFaction)
    (:execute
      (Class|SoundManagerSubsystem|PlaySFX (Subsystems|GetSoundManagerSubsystem) "ApplauseAfterKill" "0, 0, 0")
      (CallFunction|CheckPoints))))

(fn CheckPoints
  (if (>= (Variables|Default|GetequipeA) 5.0)
    (Utilities|FlowControl|DoOnce false
      (:Completed
        (CallFunction|DisplayResultGame false)))
    (elif (>= (Variables|Default|GetequipeB) 5.0)
      (Utilities|FlowControl|DoOnce false
        (:Completed
          (CallFunction|DisplayResultGame true))))))