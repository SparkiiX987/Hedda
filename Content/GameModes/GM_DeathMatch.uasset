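; Deathmatch game mode running up to three timed rounds between a player and an AI, with win or lose widgets.
; Tick counts down the round timer; NextRound destroys existing characters and respawns both, or compares points after the last round.
; AddPoint, uncalled here, shows the result when either side reaches two points.
; Obstacle moving is a print-only stub, and Tick passes zero delta to its cooldown.
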(event EventBeginPlay
  (Variables|Default|SetnumberOfRound 0.0)
  (Variables|Default|SetroundTime 1.2e+02)
  (CallFunction|NextRound))

(event EventTick
  (params (DeltaSeconds :type Float%20%28single-precision%29))
  (bind _timer (Variables|Default|Gettimer))
  (CallFunction|DecrementCooldown 0.0)
  (if (>= _timer 0.0)
    (CallFunction|DecrementTimer _timer DeltaSeconds)
    (if (<= (Variables|Default|Gettimer) 0.0)
      (CallFunction|NextRound))))

(fn ConstructionScript)

(fn DecrementTimer
  (params (_gameTime :type Float%20%28double-precision%29) (_deltaTime :type Float%20%28double-precision%29))
  (Variables|Default|Settimer (- _gameTime _deltaTime)))

(fn AddPoint
  (params (_toFirstPlayer :type Boolean))
  (if _toFirstPlayer
    (bind _result (Math|Float|IncrementFloat (Variables|Default|GetfirstPlayerPoints))
      (:%20%20
        (bind _output_get (Variables|Default|SetfirstPlayerPoints _result))
        (if (== _output_get 2.0)
          (CallFunction|DisplayResultGame true))))
    (else
      (bind _result_2 (Math|Float|IncrementFloat (Variables|Default|GetsecondPlayerPoints))
        (:%20%20
          (bind _output_get_2 (Variables|Default|SetsecondPlayerPoints _result_2))
          (if (== _output_get_2 2.0)
            (CallFunction|DisplayResultGame false)))))))

(fn DisplayResultGame
  (params (_victory :type Boolean))
  (if _victory
    (bind _returnvalue (UserInterface|CreateWidget "/Game/ArenaDeatMatch/Blueprints/UI/UW_Win.UW_Win_C"))
    (else
      (bind _returnvalue_2 (UserInterface|CreateWidget "/Game/ArenaDeatMatch/Blueprints/UI/UW_Lose.UW_Lose_C"))))
  (UserInterface|Viewport|AddtoViewport _returnvalue 0))

(fn ComparePoints
  (CallFunction|DisplayResultGame (> (Variables|Default|GetfirstPlayerPoints) (Variables|Default|GetsecondPlayerPoints))))

(fn SpawnPlayer
  (Game|SpawnActorfromClass "/Game/Character/Player/Blueprint/C_PlayerCharacter.C_PlayerCharacter_C" (Math|Transform|MakeTransform "0, 0, 0" "0, 0, 0" "1.000000,1.000000,1.000000") "Undefined" "MultiplyWithRoot" 0 0))

(fn SpawnIA
  (Game|SpawnActorfromClass "/Game/Character/C_BaseCharacter.C_BaseCharacter_C" (Math|Transform|MakeTransform "1000.000000,0.000000,0.000000" "0.000000,180.000000,0.000000" "1.000000,1.000000,1.000000") "Undefined" "MultiplyWithRoot" 0 0))

(fn MoveObstacles
  (Variables|Default|SetobstacleMoveCooldown 15.0)
  (Development|PrintText "Move Obstacles"))

(fn DecrementCooldown
  (params (_deltaTime :type Float%20%28double-precision%29))
  (bind _output_get (Variables|Default|SetobstacleMoveCooldown (- (Variables|Default|GetobstacleMoveCooldown) _deltaTime)))
  (if (<= _output_get 0.0)
    (CallFunction|MoveObstacles)))

(fn NextRound
  (if (< (Variables|Default|GetnumberOfRound) 3.0)
    (bind _result (Math|Float|IncrementFloat (Variables|Default|GetnumberOfRound))
      (:%20%20
        (Variables|Default|SetnumberOfRound _result)
        (Variables|Default|Settimer (Variables|Default|GetroundTime))
        (bind _outactors (Actor|GetAllActorsOfClass "/Game/Character/C_BaseCharacter.C_BaseCharacter_C"))
        (for _array_element _outactors
          (Actor|DestroyActor _array_element))
        (CallFunction|SpawnPlayer)
        (CallFunction|SpawnIA)))
    (else
      (CallFunction|ComparePoints))))