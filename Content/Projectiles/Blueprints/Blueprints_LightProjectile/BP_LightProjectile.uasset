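; BP_LightProjectile is a projectile that damages MemberFinal body parts on impact.
; FireinDirection applies a force from shoot direction and current velocity.
; Any hit plays the impact sound and a PiouPiou or Pan particle through sound and Niagara subsystems.
; Member hits damage the part and its BaseCharacter using the part's multiplier, dismember depleted parts, then destroy the projectile; other hits leave it alive.
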(event OnComponentHit(sphereComponent)
  (params (HitComponent :type Primitive%20Component%20Object%20Reference) (OtherActor :type Actor%20Object%20Reference) (OtherComp :type Primitive%20Component%20Object%20Reference) (NormalImpulse :type Vector :default "0, 0, 0") (Hit :type Hit%20Result%20Structure%20%28by%20ref%29))
  (Class|SoundManagerSubsystem|PlaySFX (Subsystems|GetSoundManagerSubsystem) "BulletImpact" (Transformation|GetWorldLocation (Variables|Default|GetsphereComponent)))
  (CallFunction|PlayCollisionVFX)
  (bind _asmember_final (Utilities|Casting|CastToMemberFinal OtherActor))
  (bind _output_get (Variables|Default|SetAs%20Member%20Final _asmember_final))
  (Class|MemberFinal|TakeDamage _output_get 1.0)
  (Class|BaseCharacter|DealDamage (Variables|/Script/Hedda.MemberFinal|GetbaseCharacter _output_get) (* (Variables|Default|Getdamage) (Variables|/Script/Hedda.MemberFinal|GetmultiplacaterDamage _output_get)))
  (if (<= (Class|MemberFinal|GetHealthPoints _asmember_final) 0.0)
    (Class|MemberFinal|Dismember _asmember_final)
    (Actor|DestroyActor _output_get))
  (Actor|DestroyActor))

(event EventFireinDirection
  (params (_shootDirection :type Vector%20%28by%20ref%29 :default "0, 0, 0"))
  (Physics|AddForce :Force (* _shootDirection (Transformation|GetVelocity))))

(fn ConstructionScript)

(fn PlayCollisionVFX
  (if (Variables|Default|GetbIsPiouPiouProjectile)
    (Class|NiagaraSystemSubsystem|PlayParticle (Subsystems|GetNiagaraSystemSubsystem) "PiouPiouCollision" (Transformation|GetActorLocation) "0, 0, 0")
    (Development|PrintString "Hello")
    (else
      (Class|NiagaraSystemSubsystem|PlayParticle (Subsystems|GetNiagaraSystemSubsystem) "PanCollision" (Transformation|GetActorLocation) "0, 0, 0")
      (Development|PrintString "Hello")))
  (return 0.3))