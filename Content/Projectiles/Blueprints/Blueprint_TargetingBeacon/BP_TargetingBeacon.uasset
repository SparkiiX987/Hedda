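; Targeting beacon projectile that stops on hit and calls the firing character's second-slot weapon (Weapons[1]) to lob heavy projectiles onto its position.
; "Kaboum" fires one exact shot, while other weapons fire a timed salvo with random XY scatter, cancelled by a timer based on bullet count.
; Shots leave the character's HeavyProjectileSpawnPoint on a suggested custom-arc velocity.
; The first Tick copies the character's faction, then disables ticking.
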(event Custom|CallSpawnBullet
  (bind _self self)
  (bind _minoffsettarget (Variables|Default|GetminOffSetTarget))
  (bind _maxoffsettarget_0 (Variables|Default|GetmaxOffSetTarget_0))
  (bind _returnvalue (Transformation|GetActorLocation _self))
  (bind _returnvalue_2 (Math|Random|RandomFloatinRange _minoffsettarget _maxoffsettarget_0))
  (bind (_x _y _z) (Math|Vector|BreakVector _returnvalue))
  (CallFunction|SpawnBullet (Variables|/Script/Hedda.Weapon|Getprojectile (Utilities|Array|Get(acopy) (Variables|/Script/Hedda.BaseCharacter|Getweapons (stale Collision|EventHit _asc_base_character)) 1)) (Math|Transform|MakeTransform (Transformation|GetWorldLocation (Variables|/Script/Hedda.BaseCharacter|GetheavyProjectileSpawnPoint (stale Collision|EventHit _asc_base_character))) (Math|Conversions|RotationFromXVector (Math|Vector|GetForwardVector (Variables|/Script/Hedda.BaseCharacter|GetheavyProjectileSpawnPoint (stale Collision|EventHit _asc_base_character))))) (Transformation|GetWorldLocation (Variables|/Script/Hedda.BaseCharacter|GetheavyProjectileSpawnPoint (stale Collision|EventHit _asc_base_character))) (Math|Vector|MakeVector (+ _returnvalue_2 _x) (+ _returnvalue_2 _y) _z)))

(event EventBeginPlay)

(event Collision|EventActorBeginOverlap
  (params (OtherActor :type Actor%20Object%20Reference)))

(event EventTick
  (params (DeltaSeconds :type Float%20%28single-precision%29))
  (CallFunction|SetBulletFaction)
  (Actor|Tick|SetActorTickEnabled false))

(event Collision|EventHit
  (params (MyComp :type Primitive%20Component%20Object%20Reference) (Other :type Actor%20Object%20Reference) (OtherComp :type Primitive%20Component%20Object%20Reference) (bSelfMoved :type Boolean) (HitLocation :type Vector :default "0, 0, 0") (HitNormal :type Vector :default "0, 0, 0") (NormalImpulse :type Vector :default "0, 0, 0") (Hit :type Hit%20Result%20Structure%20%28by%20ref%29))
  (bind _timebetweenbullet (Variables|Default|GettimeBetweenBullet))
  (Game|Components|ProjectileMovement|SetVelocityinLocalSpace (Variables|Default|GetprojectileMovementComponent) "0, 0, 0")
  (bind _asc_base_character (Utilities|Casting|CastToC_BaseCharacter (Variables|Default|GetcharacterFrom)))
  (if (== (Utilities|String|StringToName (Variables|/Script/Hedda.Weapon|GetweaponName (Utilities|Array|Get(acopy) (Variables|/Script/Hedda.BaseCharacter|Getweapons _asc_base_character) 1))) "Kaboum")
    (CallFunction|SpawnBullet (Variables|/Script/Hedda.Weapon|Getprojectile (Utilities|Array|Get(acopy) (Variables|/Script/Hedda.BaseCharacter|Getweapons _asc_base_character) 1)) (Math|Transform|MakeTransform (Transformation|GetWorldLocation (Variables|/Script/Hedda.BaseCharacter|GetheavyProjectileSpawnPoint _asc_base_character)) (Math|Conversions|RotationFromXVector (Math|Vector|GetForwardVector (Variables|/Script/Hedda.BaseCharacter|GetheavyProjectileSpawnPoint _asc_base_character)))) (Transformation|GetWorldLocation (Variables|/Script/Hedda.BaseCharacter|GetheavyProjectileSpawnPoint _asc_base_character)) (Transformation|GetActorLocation self))
    (else
      (bind _returnvalue (Utilities|Time|SetTimerbyEvent (delegate Custom|CallSpawnBullet) _timebetweenbullet true))
      (Variables|Default|SettimerBullet _returnvalue)
      (Utilities|Time|SetTimerbyFunctionName 0 "CancelShoot" (+ (* _timebetweenbullet (Variables|/Script/Hedda.Weapon|GetbulletNumber (Utilities|Array|Get(acopy) (Variables|/Script/Hedda.BaseCharacter|Getweapons _asc_base_character) 1))) 0.1)))))

(fn ConstructionScript)

(fn SetBulletFaction
  (bind _asc_base_character (Utilities|Casting|CastToC_BaseCharacter (Variables|Default|GetcharacterFrom)))
  (Variables|Default|SetbulletFaction (Default|GetFaction _asc_base_character)))

(fn SpawnBullet
  (params (projectile :type Actor%20Class%20Reference) (spawnTransform :type Transform) (startPos :type Vector) (endPos :type Vector))
  (bind _returnvalue (Game|SpawnActorfromClass projectile spawnTransform "Undefined" "MultiplyWithRoot" 0 0))
  (Utilities|IsValid _returnvalue
    (:Is%20Valid
      (bind _asbp_heavy_projectile (Utilities|Casting|CastToBP_HeavyProjectile _returnvalue))
      (Variables|Default|SetbulletFaction (Variables|Default|GetbulletFaction))
      (bind _outlaunchvelocity (Game|SuggestProjectileVelocityCustomArc startPos endPos 0.0 0.5))
      (Variables|/Script/Engine.MovementComponent|SetVelocity (Variables|/Script/Hedda.FPSProjectile|GetprojectileMovementComponent _asbp_heavy_projectile) _outlaunchvelocity))
    (:Is%20Not%20Valid
      (Development|PrintString "heavy projectile not valid"))))

(fn CancelShoot
  (Utilities|Time|ClearandInvalidateTimerbyHandle (Variables|Default|GettimerBullet)))