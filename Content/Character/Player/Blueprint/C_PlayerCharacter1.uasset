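; Player character Blueprint that routes Enhanced Input to movement, head look, light and heavy shooting, dash and pause menu.
; Widget components display health, ammo and heavy-shot reload, refreshed on damage, firing and Tick.
; A dynamic material on the dash HUD module signals cooldown, and starting to move can randomly trigger a gas leak.
; Death extends parent logic with a death screen showing the respawn countdown until it expires.
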(event Input|EnhancedActionEvents|EnhancedInputActionIA_Move
  (params (ActionValue :type Vector%202D%20Structure) (ElapsedSeconds :type Float%20%28double-precision%29) (TriggeredSeconds :type Float%20%28double-precision%29) (InputAction :type Input%20Action%20Object%20Reference :default "/Game/Inputs/InputActions/IA_Move.IA_Move"))
  (bind _returnvalue (Pawn|GetControlRotation :!class /Script/Engine.Pawn))
  (bind _returnvalue_2 (Pawn|GetControlRotation :!class /Script/Engine.Pawn))
  (:Triggered
    (Pawn|Input|AddMovementInput (Math|Vector|GetForwardVector (Math|Rotator|MakeRotator (.roll _returnvalue_2) 0.0 (.yaw _returnvalue_2))) (.x ActionValue) false)
    (Pawn|Input|AddMovementInput (Math|Vector|GetRightVector (Math|Rotator|MakeRotator (.roll _returnvalue) 0.0 (.yaw _returnvalue))) (.y ActionValue) false)
    (if (not (Variables|Default|GetisMoving))
      (Variables|Default|SetisMoving true)
      (if (<= (Math|Random|RandomFloatinRange 0.0 1e+02) (Variables|Default|GetPercentOfChance))
        (CallFunction|LeakGas))))
  (:Completed
    (Variables|Default|SetisMoving false)))

(event Input|EnhancedActionEvents|EnhancedInputActionIA_PauseMenu
  (params (ActionValue :type Boolean) (ElapsedSeconds :type Float%20%28double-precision%29) (TriggeredSeconds :type Float%20%28double-precision%29) (InputAction :type Input%20Action%20Object%20Reference :default "/Game/Inputs/InputActions/IA_PauseMenu.IA_PauseMenu"))
  (if (UserInterface|Viewport|IsinViewport (Variables|Default|GetpauseMenuRef))
    (Game|SetGamePaused false)
    (Widget|RemovefromParent (Variables|Default|GetpauseMenuRef))
    (Variables|/Script/Engine.PlayerController|SetbShowMouseCursor (Game|GetPlayerController 0) false)
    (else
      (Game|SetGamePaused true)
      (bind _returnvalue (UserInterface|CreateWidget "/Game/Menus/Blueprints/UW_PauseMenu.UW_PauseMenu_C"))
      (bind _output_get (Variables|Default|SetpauseMenuRef _returnvalue))
      (UserInterface|Viewport|AddtoViewport _output_get 0)
      (Variables|/Script/Engine.PlayerController|SetbShowMouseCursor (Game|GetPlayerController 0) true))))

(event Input|EnhancedActionEvents|EnhancedInputActionIA_Look
  (params (ActionValue :type Vector%202D%20Structure) (ElapsedSeconds :type Float%20%28double-precision%29) (TriggeredSeconds :type Float%20%28double-precision%29) (InputAction :type Input%20Action%20Object%20Reference :default "/Game/Inputs/InputActions/IA_Look.IA_Look"))
  (Class|BaseCharacter|RotateHead ActionValue)
  (Variables|Default|SetbodyRotationSpeed (Math|Float|Absolute(Float) (.X (Math|Vector2D|BreakVector2D ActionValue)))))

(event Input|EnhancedActionEvents|EnhancedInputActionIA_HeavyAttack
  (params (ActionValue :type Boolean) (ElapsedSeconds :type Float%20%28double-precision%29) (TriggeredSeconds :type Float%20%28double-precision%29) (InputAction :type Input%20Action%20Object%20Reference :default "/Game/Inputs/InputActions/IA_HeavyAttack.IA_HeavyAttack"))
  (CallFunction|HeavyShoot))

(event Input|EnhancedActionEvents|EnhancedInputActionIA_LightAttack
  (params (ActionValue :type Boolean) (ElapsedSeconds :type Float%20%28double-precision%29) (TriggeredSeconds :type Float%20%28double-precision%29) (InputAction :type Input%20Action%20Object%20Reference :default "/Game/Inputs/InputActions/IA_LightAttack.IA_LightAttack"))
  (:Triggered
    (CallFunction|LightShoot :!label _label)
    (Default|FirstWeaponDecresse (Variables|Default|GetWeaponsWidget) (Math|Conversions|ToFloat(Integer) (Variables|Default|GetbulletLightShot)) (Math|Conversions|ToFloat(Integer) (Variables|Default|GetbulletsLightMax))))
  (:Started
    (goto _label)))

(event Input|EnhancedActionEvents|EnhancedInputActionIA_Dash
  (params (ActionValue :type Boolean) (ElapsedSeconds :type Float%20%28double-precision%29) (TriggeredSeconds :type Float%20%28double-precision%29) (InputAction :type Input%20Action%20Object%20Reference :default "/Game/Inputs/InputActions/IA_Dash.IA_Dash"))
  (CallFunction|Dash)
  (Rendering|Material|SetScalarParameterValue (Variables|Default|GetDiodeMaterial) "X" 0.5 :!class /Script/Engine.MaterialInstanceDynamic)
  (Rendering|Material|SetScalarParameterValue (Variables|Default|GetDiodeMaterial) "Y" 0.5 :!class /Script/Engine.MaterialInstanceDynamic))

(event EventBeginPlay
  (|CallParentFunction)
  (for _index (range 0 6)
    (CallFunction|InitializeMembers _index))
  (bind _asplayer_controller (Utilities|Casting|CastToPlayerController (Pawn|GetController)))
  (Utilities|IsValid (PlayerController|LocalPlayerSubsystems|GetEnhancedInputLocalPlayerSubsystem _asplayer_controller)
    (:Is%20Valid
      (Input|AddMappingContext (PlayerController|LocalPlayerSubsystems|GetEnhancedInputLocalPlayerSubsystem _asplayer_controller) "/Game/Inputs/IMC_PlayerInputs.IMC_PlayerInputs" 0 "(bIgnoreAllPressedKeysUntilRelease=True,bForceImmediately=False,bNotifyUserSettings=False)")
      (bind _asuwb_munitions (Utilities|Casting|CastToUWB_Munitions (UserInterface|GetWidget (Variables|Default|GetAmmo))))
      (Variables|Default|SetWeaponsWidget _asuwb_munitions)
      (bind _asuwb_health (Utilities|Casting|CastToUWB_Health (UserInterface|GetWidget (Variables|Default|GetHealth))))
      (Variables|Default|SetHealthBarWidget _asuwb_health)
      (bind _asuwb_secondary (Utilities|Casting|CastToUWB_Secondary (UserInterface|GetWidget (Variables|Default|GetSecondary))))
      (bind _output_get (Variables|Default|SetAs%20UWB%20Secondary _asuwb_secondary))
      (Default|ResetMunition _output_get)
      (CallFunction|UpdateHealthBar)
      (CallFunction|SetMuntionBar)
      (bind _returnvalue (Rendering|Material|CreateDynamicMaterialInstance (Variables|Default|Gethud_dash_lo__1_) 0 "/Game/Character/Player/Materials/Modules/M_ModuleDash.M_ModuleDash" "None" :!class /Script/Engine.PrimitiveComponent))
      (Variables|Default|SetDiodeMaterial _returnvalue))))

(event EventDealDamage
  (params (_amount :type Float%20%28single-precision%29) (_bFromPlayer :type Boolean) (instagator :type Actor%20Object%20Reference))
  (|CallParentFunction _amount false 0)
  (CallFunction|UpdateHealthBar))

(event EventTick
  (params (DeltaSeconds :type Float%20%28single-precision%29))
  (bind _diodematerial (Variables|Default|GetDiodeMaterial))
  (bind _timerbeforerespawn (Variables|Default|GetTimerBeforeRespawn))
  (|CallParentFunction DeltaSeconds)
  (CallFunction|ReloadUI 0.0)
  (if (Variables|Default|GetbIsDead)
    (Default|SetTimerText (stale EventDeath _returnvalue) _timerbeforerespawn)
    (if (<= _timerbeforerespawn 0.0)
      (Widget|RemovefromParent (stale EventDeath _returnvalue))
      (if (<= (Variables|Default|GetdashCooldown) 0.0) :!label _label
        (Utilities|IsValid _diodematerial
          (:Is%20Valid
            (Rendering|Material|SetScalarParameterValue _diodematerial "X" 0.0 :!class /Script/Engine.MaterialInstanceDynamic)
            (Rendering|Material|SetScalarParameterValue (Variables|Default|GetDiodeMaterial) "Y" 0.0 :!class /Script/Engine.MaterialInstanceDynamic)))))
    (else
      (goto _label))))

(event EventUpdateHealthBar
  (Default|SetHealtBar (Variables|Default|GetHealthBarWidget)))

(event EventDeath
  (params (bByPlayer :type Boolean))
  (if (not (Variables|Default|GetbIsDead))
    (|CallParentFunction false)
    (bind _returnvalue (UserInterface|CreateWidget "/Game/Menus/Blueprints/UWB_DeathScreen.UWB_DeathScreen_C" (Game|GetPlayerController 0)))
    (UserInterface|Viewport|AddtoViewport _returnvalue 0)))

(fn ConstructionScript
  (|CallParentFunction))

(fn ReloadUI
  (params (DeltaTime :type Float%20%28double-precision%29))
  (Default|ReloadBar (Variables|Default|GetAs%20UWB%20Secondary) (Variables|Default|GetreloadTimerHeavy) (Variables|Default|GetreloadTimeHeavy)))

(fn SetMuntionBar
  (Default|ResetMunition (Variables|Default|GetWeaponsWidget)))

(fn HeavyAttackCooldown
  (Default|SecondWeaponDecress (Variables|Default|GetWeaponsWidget) (Variables|Default|GetreloadTimerHeavy) (Variables|Default|GetreloadTimeHeavy)))