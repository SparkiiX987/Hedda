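; C_AssaultAI is an AI character Blueprint for an assault unit, built on a parent class that handles construction and body lookup.
; It passes its faction to both the parent and its AIController, and supplies fixed ideal attack and defend radii.
; Zone functions are stubs: GoToZone does nothing, its disconnected loop for claiming a zone through the Blackboard never runs, and the free-zone query always returns false.
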(fn ConstructionScript
  (|CallParentFunction))

(fn GotoZone)

(fn SetFaction
  (params (Faction :type Faction%20Enum :default "NewEnumerator0"))
  (|CallParentFunction Faction)
  (Variables|/Game/Character/AI/Controller/BP_AIController.BP_AIController_C|SetFaction (Variables|Default|GetAIController) Faction))

(fn GetIdealRange
  (return 1.5e+02 5e+02))

(fn GetFreeZone
  (params (Actor :type C%20Assault%20AI%20Object%20Reference))
  (return false 0))

(fn GetEnemiinZone
  (params (Self%20Actor :type C%20Base%20Character%20Object%20Reference))
  (return 0))

(fn GetBody
  (return (|CallParentFunction)))