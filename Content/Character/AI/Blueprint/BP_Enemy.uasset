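; AI-controlled arena enemy that extends a parent character with aiming, zone selection and combat cooldowns.
; While alive, Tick counts down weapon and dash timers, derives yaw from movement, and smoothly aims at a body member of the controller's attack target with a pitch offset.
; GoToZone picks a GM_Arena zone into the blackboard and notifies it.
; Faction passes to BP_AIController, and DealDamage raises an AI damage-sense event.
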(event EventBeginPlay
  (|CallParentFunction)
  (bind _asgm_arena (Utilities|Casting|CastToGM_Arena (Game|GetGameMode)))
  (Variables|Default|SetGameMode _asgm_arena)
  (bind _asbp_aicontroller (Utilities|Casting|CastToBP_AIController (AI|GetAIController self)))
  (Variables|Default|SetAIController _asbp_aicontroller))

(event EventDealDamage
  (params (_amount :type Float%20%28single-precision%29))
  (|CallParentFunction _amount)
  (Class|AISenseDamage|ReportDamageEvent 0 self _amount (Transformation|GetActorLocation) "0, 0, 0" "None"))

(event EventTick
  (params (DeltaSeconds :type Float%20%28single-precision%29))
  (bind _returnvalue (Transformation|GetActorTransform))
  (bind _aicontroller (Variables|Default|GetAIController))
  (bind _attack_target (Variables|/Game/Character/AI/Controller/BP_AIController.BP_AIController_C|GetAttack%20Target _aicontroller))
  (bind _membersfinals (Variables|/Script/Hedda.BaseCharacter|GetmembersFinals _attack_target))
  (bind _output (Utilities|Array|Get(acopy) _membersfinals 2))
  (bind _returnvalue_2 (Transformation|GetWorldLocation _output))
  (bind _returnvalue_3 (Math|Rotator|FindRelativeLookatRotation _returnvalue _returnvalue_2))
  (if (not (Variables|Default|GetbIsDead))
    (|SetTImer DeltaSeconds
      (:exec
        (Utilities|IsValid (Variables|Default|GetAIController)
          (:Is%20Valid
            (bind _output_get (Variables|Default|SetYawRotation (Class|KismetAnimationLibrary|CalculateDirection (Transformation|GetVelocity) (Transformation|GetActorRotation))))
            (Utilities|IsValid (Variables|/Game/Character/AI/Controller/BP_AIController.BP_AIController_C|GetAttack%20Target (Variables|Default|GetAIController))
              (:Is%20Valid
                (Variables|Default|SetRotatorToEnemies (Math|Interpolation|RInterpTo (Variables|Default|GetRotatorToEnemies) (Math|Rotator|MakeRotator (.roll _returnvalue_3) (+ (.pitch _returnvalue_3) 4e+01) (.yaw _returnvalue_3)) DeltaSeconds 5.0)))
              (:Is%20Not%20Valid
                (Variables|Default|SetRotatorToEnemies (Math|Rotator|MakeRotator 0.0 0.0 _output_get))))))))))

(fn ConstructionScript
  (|CallParentFunction))

(fn GotoZone
  (bind _aicontroller (Variables|Default|GetAIController))
  (bind _array_element (Utilities|Array|ForEachLoopwithBreak (Variables|/Game/GameModes/GM_Arena.GM_Arena_C|GetZone (Variables|Default|GetGameMode)) :!label _label)
    (:LoopBody
      (bind _bool (Class|BPIEnemyAI|GetFreeZone(Message) _array_element self))
      (Development|PrintString (Utilities|String|ToString(Boolean) _bool))
      (if _bool
        (goto _label)
        (else
          (AI|Components|Blackboard|SetValueasObject (AI|GetBlackboard _aicontroller) (Variables|/Game/Character/AI/Controller/BP_AIController.BP_AIController_C|GetCurrentZone _aicontroller) _array_element)
          (Class|BPIEnemyAI|GoIntoZone(Message) _array_element self)
          (goto _label Break))))))

(fn SetFaction
  (params (Faction :type Faction%20Enum :default "NewEnumerator0"))
  (|CallParentFunction Faction)
  (Variables|/Game/Character/AI/Controller/BP_AIController.BP_AIController_C|SetFaction (Variables|Default|GetAIController) Faction))

(fn GetIdealRange
  (return 1.5e+02 5e+02))

(fn GetFreeZone
  (params (Actor :type BP%20Enemy%20Object%20Reference))
  (return false 0))

(fn GetEnemiinZone
  (params (Self%20Actor :type C%20Base%20Character%20Object%20Reference))
  (return 0))

(fn GetBody
  (return (|CallParentFunction)))