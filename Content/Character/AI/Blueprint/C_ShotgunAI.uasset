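; C_ShotgunAI is an AI character Blueprint, named for a shotgun enemy type, that extends a parent character with AI hooks.
; Taking damage runs the parent logic, then reports a damage event for AI perception with itself as instigator.
; Setting the faction also copies it to the AI controller.
; Zone and ideal-range queries are stubs returning empty values, while GetBody defers to the parent.
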(event EventDealDamage
  (params (_amount :type Float%20%28single-precision%29))
  (|CallParentFunction _amount)
  (Class|AISenseDamage|ReportDamageEvent 0 self _amount (Transformation|GetActorLocation) "0, 0, 0" "None"))

(fn ConstructionScript
  (|CallParentFunction))

(fn SetFaction
  (params (Faction :type Faction%20Enum :default "NewEnumerator0"))
  (|CallParentFunction Faction)
  (Variables|/Game/Character/AI/Controller/BP_AIController.BP_AIController_C|SetFaction (Variables|Default|GetAIController) Faction))

(fn GetBody
  (return (|CallParentFunction)))

(fn GetEnemiinZone
  (params (Self%20Actor :type C%20Base%20Character%20Object%20Reference))
  (return 0))

(fn GetFreeZone
  (params (Actor :type C%20Assault%20AI%20Object%20Reference))
  (return false 0))

(fn GetIdealRange
  (return 0.0 0.0))