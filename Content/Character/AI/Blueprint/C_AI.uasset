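; AI-controlled arena character that extends a parent character with targeting, faction and damage hooks for BP_AIController.
; While alive, Tick counts down reload, fire-delay and dash timers, then smoothly turns RotatorToEnemies toward the controller's attack target with a pitch offset, falling back to movement direction.
; Damage is reported as an AI sense event, and faction changes propagate to the controller.
; GetEnemiInZone, GetFreeZone and GetIdealRange are empty stubs here.
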(event EventBeginPlay
  (|CallParentFunction)
  (bind _asgm_arena (Utilities|Casting|CastToGM_Arena (Game|GetGameMode)))
  (Variables|Default|SetGameMode _asgm_arena)
  (bind _asbp_aicontroller (Utilities|Casting|CastToBP_AIController (AI|GetAIController self)))
  (Variables|Default|SetAIController _asbp_aicontroller))

(event EventDealDamage
  (params (_amount :type Float%20%28single-precision%29) (_bFromPlayer :type Boolean) (instagator :type Actor%20Object%20Reference))
  (|CallParentFunction _amount _bFromPlayer instagator)
  (Class|AISenseDamage|ReportDamageEvent self instagator _amount (Transformation|GetActorLocation) "0, 0, 0" "None"))

(event EventTick
  (params (DeltaSeconds :type Float%20%28single-precision%29))
  (bind _returnvalue (Transformation|GetActorTransform))
  (bind _aicontroller (Variables|Default|GetAIController))
  (bind _attack_target (Variables|/Game/Character/AI/Controller/BP_AIController.BP_AIController_C|GetAttack%20Target _aicontroller))
  (bind _membersfinals (Variables|/Script/Hedda.BaseCharacter|GetmembersFinals _attack_target))
  (bind _output (Utilities|Array|Get(acopy) _membersfinals 2))
  (bind _returnvalue_2 (Transformation|GetWorldLocation _output))
  (bind _returnvalue_3 (Math|Rotator|FindRelativeLookatRotation _returnvalue _returnvalue_2))
  (if (not (Variables|Default|GetbIsDead))
    (|SetTImer DeltaSeconds
      (:exec
        (Utilities|IsValid (Variables|Default|GetAIController)
          (:Is%20Valid
            (bind _output_get (Variables|Default|SetYawRotation (Class|KismetAnimationLibrary|CalculateDirection (Transformation|GetVelocity) (Transformation|GetActorRotation))))
            (Utilities|IsValid (Variables|/Game/Character/AI/Controller/BP_AIController.BP_AIController_C|GetAttack%20Target (Variables|Default|GetAIController))
              (:Is%20Valid
                (Variables|Default|SetRotatorToEnemies (Math|Interpolation|RInterpTo (Variables|Default|GetRotatorToEnemies) (Math|Rotator|MakeRotator (.roll _returnvalue_3) (+ (.pitch _returnvalue_3) 45.0) (.yaw _returnvalue_3)) DeltaSeconds 5.0)))
              (:Is%20Not%20Valid
                (Variables|Default|SetRotatorToEnemies (Math|Rotator|MakeRotator 0.0 0.0 _output_get))))))))))

(fn ConstructionScript
  (|CallParentFunction))

(fn SetFaction
  (params (Faction :type Faction%20Enum :default "NewEnumerator0"))
  (|CallParentFunction Faction)
  (Variables|/Game/Character/AI/Controller/BP_AIController.BP_AIController_C|SetFaction (Variables|Default|GetAIController) Faction))

(fn GetEnemiinZone
  (params (Self%20Actor :type C%20Base%20Character%20Object%20Reference))
  (return 0))

(fn GetFreeZone
  (params (Actor :type C%20Assault%20AI%20Object%20Reference))
  (return false 0))

(fn GetIdealRange
  (return 0.0 0.0))