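; Base mecha character for the arena, built from seven linked MemberFinal child actors, with faction, health and two weapons.
; Weapon data sets light-shot fire rate, ammo and reload plus heavy-shot cooldown, with empty functions for ammo and cooldown display.
; Death triggers ragdoll, unpossesses, updates kill/death counts and requests a GM_Arena respawn.
; Tick runs timers, random gas leaks and sparks keyed to player 0's health rather than its own.
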(event EventBeginPlay
  (CallFunction|SetStat)
  (for _index (range 0 6)
    (CallFunction|InitializeMembers _index)))

(event EventDeath
  (params (bByPlayer :type Boolean))
  (if (not (Variables|Default|GetbIsDead))
    (Physics|SetSimulatePhysics (Variables|Character|GetMesh) true)
    (Variables|/Script/Engine.MovementComponent|SetVelocity (Variables|Character|GetCharacterMovement) "0, 0, 0")
    (Variables|Default|SetTimerBeforeRespawn 5.0)
    (Variables|Default|SetbIsDead true)
    (CallFunction|IncrementKills bByPlayer)
    (CallFunction|IncrementDeaths)
    (Pawn|UnPossess (Pawn|GetController))
    (Class|SoundManagerSubsystem|PlaySFX (Subsystems|GetSoundManagerSubsystem) "MechaDeathExplosion" (Transformation|GetActorLocation self))
    (Utilities|FlowControl|Delay 5.0)
    (bind _currentzone (Variables|Default|GetCurrentZone)
      (:then
        (Default|ExitZone _currentzone self))
      (:else
        _))
    (bind _asgm_arena (Utilities|Casting|CastToGM_Arena (Game|GetGameMode)))
    (Default|RespawnEntity _asgm_arena self)))

(event EventTick
  (params (DeltaSeconds :type Float%20%28single-precision%29))
  (if (>= (Variables|Default|GetreloadTimerHeavy) 0.0)
    (Variables|Default|SetreloadTimerHeavy (- (Variables|Default|GetreloadTimerHeavy) DeltaSeconds))
    (CallFunction|HeavyAttackCooldown))
  (if (>= (Variables|Default|GetfireDelayLightTimer) 0.0)
    (Variables|Default|SetfireDelayLightTimer (- (Variables|Default|GetfireDelayLightTimer) DeltaSeconds)))
  (if (> (Variables|Default|GetdashCooldown) 0.0)
    (Variables|Default|SetdashCooldown (- (Variables|Default|GetdashCooldown) DeltaSeconds)))
  (CallFunction|ManageLeakGas DeltaSeconds)
  (CallFunction|ManageSparks DeltaSeconds)
  (if (Variables|Default|GetbIsDead)
    (Variables|Default|SetTimerBeforeRespawn (- (Variables|Default|GetTimerBeforeRespawn) DeltaSeconds))))

(event EventDealDamage
  (params (_amount :type Float%20%28single-precision%29) (_bFromPlayer :type Boolean) (instagator :type Actor%20Object%20Reference))
  (bind _output_get (Variables|Default|SethealPoint (- (Variables|Default|GethealPoint) _amount)))
  (if (<= _output_get 0.0)
    (Class|NiagaraSystemSubsystem|PlayParticle (Subsystems|GetNiagaraSystemSubsystem) "PurpleExplosion" "0, 0, 0" "0, 0, 0" (Variables|Default|GetCapsuleComponent))
    (Utilities|FlowControl|Delay 1.0)
    (Class|BaseCharacter|Death _bFromPlayer)))

(fn ConstructionScript
  (for _index (range 0 6)
    (CallFunction|InitializeMembers _index)
    (Variables|Default|SetPlacesToLeakGas (Utilities|Array|MakeArray (Variables|Default|GetLeakGas1) (Variables|Default|GetLeakGas2) (Variables|Default|GetLeakGas3) (Variables|Default|GetLeakGas4) (Variables|Default|GetLeakGas5) (Variables|Default|GetLeakGas6) (Variables|Default|GetLeakGas7)))
    (Variables|Default|SetInsideSparks (Utilities|Array|MakeArray (Variables|Default|GetSparks1) (Variables|Default|GetSparks3) (Variables|Default|GetSparks2) (Variables|Default|GetSparks)))
    (Variables|Default|SetOutsideSparks (Utilities|Array|MakeArray (Variables|Default|GetSparks4) (Variables|Default|GetSparks5) (Variables|Default|GetSparks6) (Variables|Default|GetSparks7) (Variables|Default|GetSparks8) (Variables|Default|GetSparks9)))))

(fn SetFaction
  (params (Faction :type Faction%20Enum :default "NewEnumerator0"))
  (Variables|Default|SetFaction Faction))

(fn GetFaction
  (return (Variables|Default|GetFaction)))

(fn LightShoot
  (bind _reloadtimelight (Variables|Default|GetreloadTimeLight))
  (bind _asmember_final (Utilities|Casting|CastToMemberFinal (Variables|/Script/Engine.ChildActorComponent|GetChildActor (Utilities|Array|Get(acopy) (Variables|Default|GetmembersFinals) 6))))
  (if (Variables|/Script/Hedda.MemberFinal|GetbCanBeUsed _asmember_final)
    (if (== (Variables|Default|GetbulletLightShot) 0)
      (if (not (Variables|Default|GetbIsReloading))
        (Variables|Default|SetbIsReloading true)
        (Utilities|Time|SetTimerbyEvent (EventDispatchers|CreateEvent :!event Reload) _reloadtimelight)
        (Variables|Default|SetreloadTimerLight _reloadtimelight))
      (elif (<= (Variables|Default|GetfireDelayLightTimer) 0.0)
        (bind _returnvalue (Class|BaseCharacter|FirstAttack))
        (CallFunction|SetBulletFaction _returnvalue)
        (Math|Integer|DecrementInt (Variables|Default|GetbulletLightShot)
          (:%20%20
            (Variables|Default|SetfireDelayLightTimer (Variables|Default|GetfireDelayLight))
            (CallFunction|SetMuntionBar)
            (Class|NiagaraSystemSubsystem|PlayParticle (Subsystems|GetNiagaraSystemSubsystem) "MuzzleShot" "0, 0, 0" "0, 0, 0" (Variables|Default|GetlightProjectileSpawnPoint))
            (switch string (Variables|/Script/Hedda.Weapon|GetweaponName (Utilities|Array|Get(acopy) (Variables|Default|Getweapons)))
              (:PiouPiou
                (Animation|PlayAnimMontage "/Game/Character/Animations/ArmsShooting/AM_ShootMecha1.AM_ShootMecha1" 1.0 "None"))
              (:PAN
                (Animation|PlayAnimMontage "/Game/Character/Animations/ArmsShooting/AM_ShootMecha2.AM_ShootMecha2" 1.1 "None")))))))))

(fn GetEnemiinZone
  (params (Self%20Actor :type C%20Base%20Character%20Object%20Reference))
  (return 0))

(fn GetIdealRange
  (return 0.0 0.0))

(fn SetStat
  (Variables|Default|SethealPoint (Variables|Default|GetmaxHealPoint))
  (Variables|Default|SetbIsDead false)
  (for (_array_element _array_index) (Variables|Default|Getweapons)
    (switch int _array_index
      (:0
        (Variables|Default|SetfireDelayLight (/ 1.0 (Variables|/Script/Hedda.Weapon|GetattackSpeed _array_element)))
        (Variables|Default|SetreloadTimeLight (Variables|/Script/Hedda.Weapon|GetreloadTime _array_element))
        (bind _output_get (Variables|Default|SetbulletsLightMax (Variables|/Script/Hedda.Weapon|Getammo _array_element)))
        (Variables|Default|SetbulletLightShot _output_get))
      (:1
        (Variables|Default|SetreloadTimeHeavy (Variables|/Script/Hedda.Weapon|GetreloadTime _array_element)))))
  (Variables|Default|SethealPoint (Variables|Default|GetmaxHealPoint)))

(fn InitializeMembers
  (params (Index :type Integer))
  (bind _membersfinals (Variables|Default|GetmembersFinals))
  (bind _asmember_final (Utilities|Casting|CastToMemberFinal (Variables|/Script/Engine.ChildActorComponent|GetChildActor (Utilities|Array|Get(acopy) _membersfinals Index))))
  (Variables|/Script/Hedda.MemberFinal|SetbodyMesh _asmember_final (Variables|Character|GetMesh))
  (Variables|/Script/Hedda.MemberFinal|SetbaseCharacter _asmember_final self)
  (switch int Index
    (:3
      (bind _asmember_final_2 (Utilities|Casting|CastToMemberFinal (Variables|/Script/Engine.ChildActorComponent|GetChildActor (Utilities|Array|Get(acopy) _membersfinals 4))))
      (Variables|/Script/Hedda.MemberFinal|SetattachedMember _asmember_final _asmember_final_2))
    (:4
      (bind _asmember_final_3 (Utilities|Casting|CastToMemberFinal (Variables|/Script/Engine.ChildActorComponent|GetChildActor (Utilities|Array|Get(acopy) _membersfinals 3))))
      (Variables|/Script/Hedda.MemberFinal|SetattachedMember _asmember_final _asmember_final_3))
    (:5
      (bind _asmember_final_4 (Utilities|Casting|CastToMemberFinal (Variables|/Script/Engine.ChildActorComponent|GetChildActor (Utilities|Array|Get(acopy) _membersfinals 6))))
      (Variables|/Script/Hedda.MemberFinal|SetattachedMember _asmember_final _asmember_final_4))
    (:6
      (bind _asmember_final_5 (Utilities|Casting|CastToMemberFinal (Variables|/Script/Engine.ChildActorComponent|GetChildActor (Utilities|Array|Get(acopy) _membersfinals 5))))
      (Variables|/Script/Hedda.MemberFinal|SetattachedMember _asmember_final _asmember_final_5))))

(fn GetBody
  (return (Utilities|Array|Get(acopy) (Variables|Default|GetmembersFinals))))

(fn HeavyShoot
  (bind _asmember_final (Utilities|Casting|CastToMemberFinal (Variables|/Script/Engine.ChildActorComponent|GetChildActor (Utilities|Array|Get(acopy) (Variables|Default|GetmembersFinals) 6))))
  (if (Variables|/Script/Hedda.MemberFinal|GetbCanBeUsed _asmember_final)
    (if (<= (Variables|Default|GetreloadTimerHeavy) 0.0)
      (bind _returnvalue (Class|BaseCharacter|SecondAttack))
      (CallFunction|SetBulletFaction _returnvalue)
      (Variables|Default|SetreloadTimerHeavy (Variables|Default|GetreloadTimeHeavy))
      (Class|NiagaraSystemSubsystem|PlayParticle (Subsystems|GetNiagaraSystemSubsystem) "HeabySmoke" "-60.000000,15.000000,215.000000" "0, 0, 0" (Variables|Default|GetCapsuleComponent)))))

(fn SetBulletFaction
  (params (NewParam :type Array%20of%20FPS%20Projectile%20Object%20References))
  (for _array_element NewParam
    (bind _asbp_base_projectile (Utilities|Casting|CastToBP_BaseProjectile _array_element))
    (Default|SetBulletFaction _asbp_base_projectile self)))

(fn ManageLeakGas
  (params (DeltaTime :type Float%20%28double-precision%29))
  (if (<= (Variables|Default|GetTimerLeakGas) 0.0)
    (CallFunction|LeakGas)
    (else
      (Variables|Default|SetTimerLeakGas (- (Variables|Default|GetTimerLeakGas) DeltaTime)))))

(fn LeakGas
  (bind _leakgasmax (Variables|Default|GetLeakGasMax))
  (bind _placestoleakgas (Variables|Default|GetPlacesToLeakGas))
  (bind _returnvalue (Math|Random|RandomInteger _leakgasmax))
  (Development|PrintString (Utilities|String|ToString(Integer) _returnvalue))
  (for _index (range 0 _returnvalue)
    (Class|NiagaraSystemSubsystem|PlayParticle (Subsystems|GetNiagaraSystemSubsystem) "GasLeak" "0, 0, 0" "0, 0, 0" (Utilities|Array|Get(acopy) _placestoleakgas (Math|Random|RandomInteger (Utilities|Array|Length _placestoleakgas))))
    (Class|SoundManagerSubsystem|PlaySFX (Subsystems|GetSoundManagerSubsystem) "AirPressure" (Transformation|GetActorLocation)))
  (Variables|Default|SetTimerLeakGas (Math|Random|RandomFloatinRange (Variables|Default|GetMinDelayLeakGas) (Variables|Default|GetMaxDelayLeakGas))))

(fn SetMuntionBar)

(fn HeavyAttackCooldown)

(fn Reload
  (Variables|Default|SetbulletLightShot (Variables|Default|GetbulletsLightMax))
  (Variables|Default|SetbIsReloading false)
  (CallFunction|SetMuntionBar))

(fn IncrementKills
  (params (FromPlayer :type Boolean))
  (if FromPlayer
    (bind _asgi_select_game_instance (Utilities|Casting|CastToGI_SelectGameInstance (Game|GetGameInstance))
      (:then
        (Math|Integer|IncrementInt (Variables|/Game/Save/Blueprint/GI_SelectGameInstance.GI_SelectGameInstance_C|GetnumbersOfKills _asgi_select_game_instance)
          (:%20%20
            _)))
      (:CastFailed
        _)))
  (return))

(fn IncrementDeaths
  (if (== self (Game|GetPlayerCharacter 0))
    (bind _asgi_select_game_instance (Utilities|Casting|CastToGI_SelectGameInstance (Game|GetGameInstance))
      (:then
        (Math|Integer|IncrementInt (Variables|/Game/Save/Blueprint/GI_SelectGameInstance.GI_SelectGameInstance_C|GetnumbersOfDeath _asgi_select_game_instance)
          (:%20%20
            _)))
      (:CastFailed
        _)))
  (return))

(fn ManageSparks
  (params (_deltaTime :type Float%20%28double-precision%29))
  (if (<= (Variables|Default|GetLaunchSparksTimer) 0.0)
    (CallFunction|LaunchSparksInside)
    (CallFunction|LaunchSparksOutside)
    (Variables|Default|SetLaunchSparksTimer 5.0)
    (else
      (Variables|Default|SetLaunchSparksTimer (- (Variables|Default|GetLaunchSparksTimer) _deltaTime)))))

(fn LaunchSparksInside
  (bind _asc_player_character (Utilities|Casting|CastToC_PlayerCharacter (Game|GetPlayerCharacter 0)))
  (if (>= (/ (- (Variables|/Script/Hedda.BaseCharacter|GetmaxHealPoint _asc_player_character) (Variables|/Script/Hedda.BaseCharacter|GethealPoint _asc_player_character)) (Variables|/Script/Hedda.BaseCharacter|GetmaxHealPoint _asc_player_character)) 0.7)
    (for _index (range 0 (- (Utilities|Array|Length (Variables|Default|GetInsideSparks)) (Math|Float|Truncate (* (- 1.0 (/ (- (Variables|/Script/Hedda.BaseCharacter|GetmaxHealPoint _asc_player_character) (Variables|/Script/Hedda.BaseCharacter|GethealPoint _asc_player_character)) (Variables|/Script/Hedda.BaseCharacter|GetmaxHealPoint _asc_player_character))) 1e+01))))
      (Class|NiagaraSystemSubsystem|PlayParticle (Subsystems|GetNiagaraSystemSubsystem) "SparksLil" "0, 0, 0" "0, 0, 0" (Utilities|Array|Get(acopy) (Variables|Default|GetInsideSparks) (Math|Random|RandomInteger (- (Utilities|Array|Length (Variables|Default|GetInsideSparks)) (Math|Float|Truncate (* (- 1.0 (/ (- (Variables|/Script/Hedda.BaseCharacter|GetmaxHealPoint _asc_player_character) (Variables|/Script/Hedda.BaseCharacter|GethealPoint _asc_player_character)) (Variables|/Script/Hedda.BaseCharacter|GetmaxHealPoint _asc_player_character))) 1e+01)))))))))

(fn LaunchSparksOutside
  (bind _asc_player_character (Utilities|Casting|CastToC_PlayerCharacter (Game|GetPlayerCharacter 0)))
  (if (>= (/ (- (Variables|/Script/Hedda.BaseCharacter|GetmaxHealPoint _asc_player_character) (Variables|/Script/Hedda.BaseCharacter|GethealPoint _asc_player_character)) (Variables|/Script/Hedda.BaseCharacter|GetmaxHealPoint _asc_player_character)) 0.7)
    (for _index (range 0 (- (Utilities|Array|Length (Variables|Default|GetOutsideSparks)) (Math|Float|Truncate (* (- 1.0 (/ (- (Variables|/Script/Hedda.BaseCharacter|GetmaxHealPoint _asc_player_character) (Variables|/Script/Hedda.BaseCharacter|GethealPoint _asc_player_character)) (Variables|/Script/Hedda.BaseCharacter|GetmaxHealPoint _asc_player_character))) 1e+01))))
      (Class|NiagaraSystemSubsystem|PlayParticle (Subsystems|GetNiagaraSystemSubsystem) "SparksMid" "0, 0, 0" "0, 0, 0" (Utilities|Array|Get(acopy) (Variables|Default|GetOutsideSparks) (Math|Random|RandomInteger (- (Utilities|Array|Length (Variables|Default|GetOutsideSparks)) (Math|Float|Truncate (* (- 1.0 (/ (- (Variables|/Script/Hedda.BaseCharacter|GetmaxHealPoint _asc_player_character) (Variables|/Script/Hedda.BaseCharacter|GethealPoint _asc_player_character)) (Variables|/Script/Hedda.BaseCharacter|GetmaxHealPoint _asc_player_character))) 1e+01)))))))))