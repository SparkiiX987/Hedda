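; BP_Zone is a zone actor that tracks up to two occupying entities, apparently for faction-based AI combat positioning.
; Enter and exit events maintain the occupant array, and GetEnemiInZone returns the other occupant to a member.
; GetFreeZone compares an actor's faction with an occupant's, returning the result with the zone.
; Tick draws the box bounds for debugging, while GetIdealRange returns only zero radii and the team-check graph is unwired.
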(event EventExitZone
  (params (Entity :type C%20Base%20Character%20Object%20Reference))
  (if (Utilities|Array|ContainsItem (Variables|Default|GetEntity) Entity)
    (Utilities|Array|RemoveItem (Variables|Default|GetEntity) Entity)))

(event EventTick
  (params (DeltaSeconds :type Float%20%28single-precision%29))
  (Rendering|Debug|DrawDebugBox (Transformation|GetActorLocation self) (Components|Box|GetScaledBoxExtent (Variables|Default|GetBox)) "(R=0.515625,G=0.000000,B=0.330865,A=1.000000)" "0, 0, 0" 0.0 1e+01))

(event EventGoIntoZone
  (params (Actor :type C%20Base%20Character%20Object%20Reference))
  (if (< (Utilities|Array|Length (Variables|Default|GetEntity)) 2)
    (Utilities|Array|Add (Variables|Default|GetEntity) Actor)))

(fn ConstructionScript)

(fn GetEnemiinZone
  (params (Self%20Actor :type C%20Base%20Character%20Object%20Reference))
  (if (Utilities|Array|ContainsItem (Variables|Default|GetEntity) Self%20Actor)
    (bind _array_element (Utilities|Array|ForEachLoopwithBreak (Variables|Default|GetEntity) :!label _label)
      (:LoopBody
        (if (!= _array_element Self%20Actor)
          (Utilities|FlowControl|Sequence
            (:then_0
              (return _array_element))
            (:then_1
              (goto _label Break))))))))

(fn GetFreeZone
  (params (Actor :type BP%20Enemy%20Object%20Reference))
  (bind _self self)
  (bind _entity (Variables|Default|GetEntity))
  (LocalVariables|SetActor%20 Actor)
  (if (< (Utilities|Array|Length _entity) 2)
    (bind _array_element (Utilities|Array|ForEachLoopwithBreak _entity)
      (:LoopBody
        (if (Utilities|Enum|Equal(Enum) (Default|GetFaction _array_element) (Default|GetFaction (LocalVariables|GetActor%20)))
          _
          (else
            (return false _self))))))
  (return (Utilities|Enum|Equal(Enum) (Default|GetFaction _array_element) (Default|GetFaction (LocalVariables|GetActor%20))) _self))

(fn GetIdealRange
  (return 0.0 0.0))